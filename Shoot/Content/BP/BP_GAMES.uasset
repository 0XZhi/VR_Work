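; BP_GAMES is a spawner Blueprint that continuously creates monsters at two preset transforms, 怪物A位置 and 怪物B位置.
; Tick runs two parallel DoOnce branches, each spawning an actor and resetting its gate after a short random delay.
; The B branch spawns BP_怪物B, while the A branch's spawn node shows no class.
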(event EventTick
  (params (DeltaSeconds :type Float%20%28single-precision%29))
  (Utilities|FlowControl|Sequence
    (:then_0
      (Utilities|FlowControl|DoOnce false :!label _label
        (:Completed
          (Game|SpawnActorfromClass "/Game/BP/bp_怪物A.BP_怪物A_C" (Variables|Default|Get怪物A位置) "Undefined" 0 0)
          (Utilities|FlowControl|Delay (Math|Random|RandomFloatinRange 0.5 1.0))
          (goto _label Reset))))
    (:then_1
      (Utilities|FlowControl|DoOnce false :!label _label_2
        (:Completed
          (Game|SpawnActorfromClass "/Game/BP/BP_怪物B.BP_怪物B_C" (Variables|Default|Get怪物B位置) "Undefined" 0 0)
          (Utilities|FlowControl|Delay (Math|Random|RandomFloatinRange 0.5 1.0))
          (goto _label_2 Reset))))))

(fn ConstructionScript)