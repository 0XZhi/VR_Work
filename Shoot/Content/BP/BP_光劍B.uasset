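; BP_光劍B is a grabbable lightsaber that cuts monsters and changes the score.
; Pickup turns off physics on its 光劍A component.
; Blade overlaps call 被A光劍砍到 on BP_怪物A or BP_怪物B, lowering the score for A and raising it for B.
; The score lives on the first BP_光劍A tagged "S", found on each hit, and is written to the 文字物件 text render.
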(event OnComponentBeginOverlap(光劍碰撞區域)
  (params (OverlappedComponent :type Primitive%20Component%20Object%20Reference) (OtherActor :type Actor%20Object%20Reference) (OtherComp :type Primitive%20Component%20Object%20Reference) (OtherBodyIndex :type Integer) (bFromSweep :type Boolean) (SweepResult :type Hit%20Result%20Structure%20%28by%20ref%29))
  (Utilities|FlowControl|Sequence
    (:then_0
      (bind _asbp_怪物a (Utilities|Casting|CastToBP_怪物A OtherActor))
      (Default|被A光劍砍到 _asbp_怪物a)
      (bind _outactors (Actor|GetAllActorsOfClasswithTag "/Game/BP/BP_光劍A.BP_光劍A_C" "S"))
      (bind _asbp_光劍a (Utilities|Casting|CastToBP_光劍A (Utilities|Array|Get(acopy) _outactors)))
      (bind _result (Math|Integer|DecrementInt (Variables|/Game/BP/BP_光劍A.BP_光劍A_C|Get分數 _asbp_光劍a))
        (:%20%20
          (Rendering|Components|TextRender|SetText (Variables|/Script/Engine.TextRenderActor|GetTextRender (Variables|Default|Get文字物件)) (Utilities|Text|ToText(String) (Utilities|String|Append "分數：" (Utilities|String|ToString(Integer) _result)))))))
    (:then_1
      (bind _asbp_怪物b (Utilities|Casting|CastToBP_怪物B OtherActor))
      (Default|被A光劍砍到 _asbp_怪物b)
      (bind _outactors_2 (Actor|GetAllActorsOfClasswithTag "/Game/BP/BP_光劍A.BP_光劍A_C" "S"))
      (bind _asbp_光劍a_2 (Utilities|Casting|CastToBP_光劍A (Utilities|Array|Get(acopy) _outactors_2)))
      (bind _result_2 (Math|Integer|IncrementInt (Variables|/Game/BP/BP_光劍A.BP_光劍A_C|Get分數 _asbp_光劍a_2))
        (:%20%20
          (Rendering|Components|TextRender|SetText (Variables|/Script/Engine.TextRenderActor|GetTextRender (Variables|Default|Get文字物件)) (Utilities|Text|ToText(String) (Utilities|String|Append "分數：" (Utilities|String|ToString(Integer) _result_2)))))))))

(event EventPickup
  (params (AttachTo :type Scene%20Component%20Object%20Reference))
  ;[1 1 1] 抓取
  (Physics|SetSimulatePhysics (Variables|Default|Get光劍A) false))

(fn ConstructionScript)