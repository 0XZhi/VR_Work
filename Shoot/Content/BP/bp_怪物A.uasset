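; Monster A actor that flies toward a fixed point and costs the player score if the A lightsaber does not cut it first.
; On BeginPlay it moves its 怪物A component to a set relative location over a random whole-second duration, then destroys itself.
; It then finds the BP_光劍A tagged "S", deducts points from its 分數 score and prints the total.
; The 被A光劍砍到 (hit by lightsaber A) function only destroys the monster.
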(event EventBeginPlay
  (Components|MoveComponentTo (Variables|Default|Get怪物A) "-225.000000,-30.000000,250.000000" "0, 0, 0" false false (Math|Conversions|ToFloat(Integer) (Math|Random|RandomIntegerinRange 1 3)) false)
  (Actor|DestroyActor self)
  (bind _outactors (Actor|GetAllActorsOfClasswithTag "/Game/BP/BP_光劍A.BP_光劍A_C" "S"))
  (bind _asbp_光劍a (Utilities|Casting|CastToBP_光劍A (Utilities|Array|Get(acopy) _outactors)))
  (bind _output_get (Variables|/Game/BP/BP_光劍A.BP_光劍A_C|Set分數 _asbp_光劍a (- (Variables|/Game/BP/BP_光劍A.BP_光劍A_C|Get分數 _asbp_光劍a) 5)))
  (Development|PrintString (Utilities|String|ToString(Integer) _output_get)))

(fn ConstructionScript)

(fn 被A光劍砍到
  (Actor|DestroyActor self))